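; BP_Slider is a slider that turns Height or Contrast axis input into a normalized value.
; A HeightMode flag selects which axis drives OffsetSlider, which moves the Slider component along a clamped local Y track and maps its position to 0–1.
; The result is stored as HeightValue or ContrastValue, and GetSliderValue returns either one on request.
; The slider starts at the minimum end on BeginPlay.
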(event `self.ReceiveBeginPlay`
  (`SceneComponent.K2_SetRelativeLocation` (`self.Slider`) (0.0 -200.0 0.0) false false)
  (set `self.CurrentPosition` -200.0))

(event `InputAxis|Height` :consume false
  (params (AxisValue :type "Float (single-precision)"))
  (if (`self.HeightMode?`)
    (bind _normalizeposition (`self.OffsetSlider` AxisValue 6.0))
    (set `self.HeightValue` _normalizeposition)))

(event `InputAxis|Contrast` :consume false
  (params (AxisValue :type "Float (single-precision)"))
  (if (not (`self.HeightMode?`))
    (bind _normalizeposition (`self.OffsetSlider` AxisValue 6.0))
    (set `self.ContrastValue` _normalizeposition)))

(fn `GetSliderValue`
  (params (`Height?` :type Boolean))
  (returns (Value :type "Float (double-precision)"))
  (return (select `bool` `Height?` :`false` (`self.ContrastValue`) :`true` (`self.HeightValue`))))

(fn `OffsetSlider`
  (params (AxisValue :type "Float (double-precision)") (MoveSpeed :type "Float (double-precision)"))
  (returns (NormalizePosition :type "Float (double-precision)"))
  (bind _output_get (set `self.CurrentPosition` (`KismetMathLibrary.FClamp` (+ (* AxisValue MoveSpeed) (`self.CurrentPosition`)) -200.0 200.0)))
  (`SceneComponent.K2_SetRelativeLocation` (`self.Slider`) (`KismetMathLibrary.MakeVector` 0.0 _output_get) false false)
  (return (`KismetMathLibrary.MapRangeClamped` (`self.CurrentPosition`) -200.0 200.0 0.0 1.0)))

(fn `UserConstructionScript`)