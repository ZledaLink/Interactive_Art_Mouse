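; BP_GridSpawnerMaster lays out a centered grid of BP_Cylinder actors, sized by MaxX, MaxY and Spacing.
; The Construction Script builds temporary static mesh components as placeholders at each grid point, centered on the actor's origin.
; On BeginPlay it spawns a cylinder at each placeholder's world transform, passing TargetActor and the height and contrast slider references, then destroys the placeholders.
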(event `self.ReceiveBeginPlay`
  (for _array_element (`self.TempMeshArray`)
    (`|SpawnActorFromClass` "/Game/BP/BP_Cylinder.BP_Cylinder_C" (`SceneComponent.K2_GetComponentToWorld` _array_element) "AlwaysSpawn" "MultiplyWithRoot" null (`self.TargetActor`) (`self.BP_Slider_Height`) (`self.BP_Slider_Contrast`) null))
  (for _array_element_2 (`self.TempMeshArray`)
    (`ActorComponent.K2_DestroyComponent` _array_element_2)))

(fn `UserConstructionScript`
  (`KismetArrayLibrary.Array_Clear` (`self.TempMeshArray`))
  (for _index (range (`self.MaxX`))
    (set `self.TempX` _index)
    (for _index_2 (range (`self.MaxY`))
      (set `self.TempY` _index_2)
      (bind _returnvalue (`AddComponent|NODE_AddStaticMeshComponent-0` :`RelativeTransform` (`KismetMathLibrary.MakeTransform` (- (`KismetMathLibrary.MakeVector` (* (`self.TempX`) (`self.Spacing`)) (* (`self.TempY`) (`self.Spacing`))) (`KismetMathLibrary.MakeVector` (/ (* (- (`self.MaxX`) 1) (`self.Spacing`)) 2.0) (/ (* (- (`self.MaxY`) 1) (`self.Spacing`)) 2.0))))))
      (`KismetArrayLibrary.Array_Add` (`self.TempMeshArray`) _returnvalue))))